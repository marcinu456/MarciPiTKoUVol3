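; Bot projectile that, on overlapping a non-instigator BP_BotV2, applies a Gameplay Effect damage spec and destroys itself.
; BeginPlay configures material, damage via SetByCaller, and speed by OwnerClass.
; PYRO rounds are non-homing flames that grow on a timeline until destroyed.
; SNIPER rounds expire after a delay, taking speed and Cheaty-only homing from ProjectileType, while color and damage switches are fixed to Slow.
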(event `self.ReceiveBeginPlay`
  (bind _projectiletype (`self.ProjectileType`))
  (bind _base_speed (`self.Base Speed`))
  (bind _base_speed_2 (`self.Base Speed`))
  (bind _returnvalue (`KismetMathLibrary.Conv_DoubleToVector` 0.2))
  (bind _returnvalue_2 (`AbilitySystemComponent.MakeOutgoingSpec` :`self` (`self.OwnerAB`) :`GameplayEffectClass` "/Game/AI/GAS/GE_EQS_Deal_Damage.GE_EQS_Deal_Damage_C" :`Level` 1.0))
  (bind _returnvalue_3 (select `/Game/AI/E_SNIPER_AMMO` _projectiletype :`NewEnumerator0` (* _base_speed 0.5) :`NewEnumerator1` (* _base_speed 5.0) :`NewEnumerator2` (* _base_speed 2.0) :!type "Float (single-precision)"))
  (switch `/Game/AI/E_BotClass` (`self.OwnerClass`)
    (:`NewEnumerator1`
      (`|ExecutionSequence`
        (:`then_0`
          (bind _returnvalue_4 (`PrimitiveComponent.CreateDynamicMaterialInstance` (`self.Sphere`) 0 "/Game/StarterContent/Materials/M_Custom.M_Custom" "None"))
          (`MaterialInstanceDynamic.SetVectorParameterValue` _returnvalue_4 "CO" (struct :`R` 1.0 :`G` 1.0 :`A` 1.0))
          (`MaterialInstanceDynamic.SetScalarParameterValue` _returnvalue_4 "EM" 10.0)
          (`MaterialInstanceDynamic.SetScalarParameterValue` _returnvalue_4 "OP" 1.0)
          (`SceneComponent.SetRelativeScale3D` (`self.Sphere`) (`KismetMathLibrary.Conv_DoubleToVector` 0.1))
          (bind (_direction _scale) (`Timeline|PyroFlame`)
            (:`Update`
              (`MaterialInstanceDynamic.SetVectorParameterValue` _returnvalue_4 "CO" (`KismetMathLibrary.MakeColor` 1.0 (`|EaseFunction` "Linear" _scale 0.5)))
              (`MaterialInstanceDynamic.SetScalarParameterValue` _returnvalue_4 "EM" (`|EaseFunction` "Linear" _scale 100.0 1.0))
              (`MaterialInstanceDynamic.SetScalarParameterValue` _returnvalue_4 "OP" (`|EaseFunction` "Linear" _scale 0.2))
              (`SceneComponent.SetRelativeScale3D` (`self.Sphere`) (`|EaseFunction` "Linear" _scale (1.0 0.05 0.05) (7.5 1.5 1.5))))
            (:`Finished`
              (`self.K2_DestroyActor`))))
        (:`then_1`
          (bind _returnvalue_5 (`AbilitySystemBlueprintLibrary.AssignTagSetByCallerMagnitude` (`AbilitySystemComponent.MakeOutgoingSpec` :`self` (`self.OwnerAB`) :`GameplayEffectClass` "/Game/AI/GAS/GE_EQS_Deal_Damage.GE_EQS_Deal_Damage_C" :`Level` 1.0) (struct :`TagName` "EQS.DATA.P1") -5.0))
          (set `self.Effect` _returnvalue_5))
        (:`then_2`
          (set `ProjectileMovementComponent.InitialSpeed` _base_speed_2 (`self.ProjectileMovement`))
          (set `ProjectileMovementComponent.MaxSpeed` _base_speed_2 (`self.ProjectileMovement`))
          (set `ProjectileMovementComponent.HomingAccelerationMagnitude` _base_speed_2 (`self.ProjectileMovement`))
          (set `ProjectileMovementComponent.HomingTargetComponent` (`self.Homing Target Component`) (`self.ProjectileMovement`))
          (set `ProjectileMovementComponent.bIsHomingProjectile` false (`self.ProjectileMovement`)))))
    (:`NewEnumerator2`
      (`|ExecutionSequence`
        (:`then_0`
          (switch `/Game/AI/E_SNIPER_AMMO` "NewEnumerator0"
            (:`NewEnumerator0`
              (bind _returnvalue_6 (`PrimitiveComponent.CreateDynamicMaterialInstance` (`self.Sphere`) 0 "/Game/StarterContent/Materials/M_Custom.M_Custom" "None"))
              (`MaterialInstanceDynamic.SetVectorParameterValue` _returnvalue_6 "CO" (struct :`R` 1.0 :`A` 1.0))
              (`MaterialInstanceDynamic.SetScalarParameterValue` _returnvalue_6 "EM" 10.0)
              (`MaterialInstanceDynamic.SetScalarParameterValue` _returnvalue_6 "OP" 1.0)
              (`SceneComponent.SetRelativeScale3D` (`self.Sphere`) _returnvalue))
            (:`NewEnumerator1`
              (bind _returnvalue_7 (`PrimitiveComponent.CreateDynamicMaterialInstance` (`self.Sphere`) 0 "/Game/StarterContent/Materials/M_Custom.M_Custom" "None"))
              (`MaterialInstanceDynamic.SetVectorParameterValue` _returnvalue_7 "CO" (struct :`G` 1.0 :`A` 1.0))
              (`MaterialInstanceDynamic.SetScalarParameterValue` _returnvalue_7 "EM" 10.0)
              (`MaterialInstanceDynamic.SetScalarParameterValue` _returnvalue_7 "OP" 1.0)
              (`SceneComponent.SetRelativeScale3D` (`self.Sphere`) _returnvalue))
            (:`NewEnumerator2`
              (bind _returnvalue_8 (`PrimitiveComponent.CreateDynamicMaterialInstance` (`self.Sphere`) 0 "/Game/StarterContent/Materials/M_Custom.M_Custom" "None"))
              (`MaterialInstanceDynamic.SetVectorParameterValue` _returnvalue_8 "CO" (struct :`B` 1.0 :`A` 1.0))
              (`MaterialInstanceDynamic.SetScalarParameterValue` _returnvalue_8 "EM" 10.0)
              (`MaterialInstanceDynamic.SetScalarParameterValue` _returnvalue_8 "OP" 1.0)
              (`SceneComponent.SetRelativeScale3D` (`self.Sphere`) _returnvalue))))
        (:`then_1`
          (`KismetSystemLibrary.Delay` 10.0)
          (`self.K2_DestroyActor`))
        (:`then_2`
          (switch `/Game/AI/E_SNIPER_AMMO` "NewEnumerator0"
            (:`NewEnumerator0`
              (bind _returnvalue_9 (`AbilitySystemBlueprintLibrary.AssignTagSetByCallerMagnitude` _returnvalue_2 (struct :`TagName` "EQS.DATA.P1") -50.0))
              (set `self.Effect` _returnvalue_9))
            (:`NewEnumerator1`
              (bind _returnvalue_10 (`AbilitySystemBlueprintLibrary.AssignTagSetByCallerMagnitude` _returnvalue_2 (struct :`TagName` "EQS.DATA.P1") -20.0))
              (set `self.Effect` _returnvalue_10))
            (:`NewEnumerator2`
              (bind _returnvalue_11 (`AbilitySystemBlueprintLibrary.AssignTagSetByCallerMagnitude` _returnvalue_2 (struct :`TagName` "EQS.DATA.P1") -10.0))
              (set `self.Effect` _returnvalue_11))))
        (:`then_3`
          (set `ProjectileMovementComponent.InitialSpeed` _returnvalue_3 (`self.ProjectileMovement`))
          (set `ProjectileMovementComponent.MaxSpeed` _returnvalue_3 (`self.ProjectileMovement`))
          (set `ProjectileMovementComponent.HomingAccelerationMagnitude` _returnvalue_3 (`self.ProjectileMovement`))
          (set `ProjectileMovementComponent.HomingTargetComponent` (`self.Homing Target Component`) (`self.ProjectileMovement`))
          (set `ProjectileMovementComponent.bIsHomingProjectile` (select `/Game/AI/E_SNIPER_AMMO` _projectiletype :`NewEnumerator2` true) (`self.ProjectileMovement`)))))))

(event `self.Sphere.OnComponentBeginOverlap`
  (params (OverlappedComponent :type "PrimitiveComponent Object Reference") (OtherActor :type "Actor Object Reference") (OtherComp :type "PrimitiveComponent Object Reference") (OtherBodyIndex :type Integer) (bFromSweep :type Boolean) (SweepResult :type "HitResult Structure (by ref)"))
  (if (not (== OtherActor (`self.GetInstigator`)))
    (bind _asbp_bot_v2 (cast `/Game/AI/BP_BotV2` OtherActor))
    (`AbilitySystemComponent.BP_ApplyGameplayEffectSpecToSelf` (`GASCharacter.AbilitySystemComponent` _asbp_bot_v2) (`self.Effect`))
    (`self.K2_DestroyActor`)))

(fn `IsThreatTo`
  (params (`Target?` :type "/Game/AI/BP_BotV2 Object Reference"))
  (returns (Danger :type Boolean))
  (return false))

(fn `UserConstructionScript`)