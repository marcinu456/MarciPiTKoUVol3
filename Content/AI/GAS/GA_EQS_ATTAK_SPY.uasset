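; GAS melee attack ability, apparently for the spy, that damages a random BP_BotV2 just in front of the owner.
; A short forward sphere overlap finds pawns, then a set-by-caller damage spec is built from a randomly picked target's ASC and self-applied, with Random feeding both steps.
; Hit or miss, it applies a brief cooldown effect with dynamically granted tags to the owner and ends immediately.
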(event `self.K2_ActivateAbility`
  (bind _returnvalue (`self.GetOwningActorFromActorInfo`))
  (`|ExecutionSequence`
    (:`then_0`
      (bind (_outactors _returnvalue_2) (`KismetSystemLibrary.SphereOverlapActors` (+ (`Actor.K2_GetActorLocation` _returnvalue) (* (`Actor.GetActorForwardVector` _returnvalue) 50.0)) 100.0 (`|MakeArray` "ObjectTypeQuery3" :!type "EObjectTypeQuery Enum") "/Game/AI/BP_BotV2.BP_BotV2_C" (`|MakeArray` _returnvalue)))
      (if _returnvalue_2
        (bind _returnvalue_3 (`AbilitySystemBlueprintLibrary.GetAbilitySystemComponent` (`KismetArrayLibrary.Array_Random` _outactors)))
        (bind _returnvalue_4 (`AbilitySystemBlueprintLibrary.AssignTagSetByCallerMagnitude` (`AbilitySystemComponent.MakeOutgoingSpec` :`self` _returnvalue_3 :`GameplayEffectClass` "/Game/AI/GAS/GE_EQS_Deal_Damage.GE_EQS_Deal_Damage_C" :`Level` 1.0) (struct :`TagName` "EQS.DATA.P1") -110.0))
        (`AbilitySystemComponent.BP_ApplyGameplayEffectSpecToSelf` _returnvalue_3 _returnvalue_4)))
    (:`then_1`
      (bind _returnvalue_5 (`AbilitySystemBlueprintLibrary.SetDuration` (`AbilitySystemComponent.MakeOutgoingSpec` :`self` (`AbilitySystemBlueprintLibrary.GetAbilitySystemComponent` (`self.GetOwningActorFromActorInfo`)) :`GameplayEffectClass` "/Game/AI/GAS/GE_EQS_COOLDOWN.GE_EQS_COOLDOWN_C" :`Level` 1.0) 1.0))
      (bind _returnvalue_6 (`AbilitySystemBlueprintLibrary.AddGrantedTags` _returnvalue_5 (`self.New Gameplay Tags`)))
      (`AbilitySystemComponent.BP_ApplyGameplayEffectSpecToSelf` (`AbilitySystemBlueprintLibrary.GetAbilitySystemComponent` (`self.GetOwningActorFromActorInfo`)) _returnvalue_6))
    (:`then_2`
      (`self.K2_EndAbility`))))